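; BP_Coaster is the rollercoaster ride actor that travels along a spline track, with hold-to-look camera control and clamped health.
; Each Tick derives speed from squared pitch-based gravity, velocity boosts and braking, then advances a looping spline distance to place the actor.
; Events set boosts, brakes, minimum speed and climbing, which replaces gravity with interpolation toward climb speed.
; Speed feeds widget text and track-sound parameters, while climbing can crossfade to its own sound.
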(event EventBeginPlay
  ;[1 1 1] BeginPlay
  (Utilities|FlowControl|Sequence
    (:then_0
      (Variables|Default|SetSplineLength (Spline|GetSplineLength (Variables|/Game/Assets/Rollercoaster/_Main/TrackSpline.TrackSpline_C|GetSpline (Variables|Default|GetSplineActor))))
      (Audio|Components|Audio|Play (Variables|Default|GetTrackSound) 0.0)
      (Variables|Default|SettxtMinSpeed (Utilities|Text|ToText(Float) (Variables|Default|GetMinSpeed) "HalfToEven" false true 1 324 0 1))
      (bind _outactors (Actor|GetAllActorsOfClass "/Game/Assets/Rollercoaster/_Main/Trigger_WarpPoint.Trigger_WarpPoint_C"))
      (Variables|Default|SetWarpPoints _outactors))
    (:then_1
      (if false ; Debug
        (Variables|Default|SetCurrentSpeed 3e+02)
        (Variables|Default|SetDistance 5.8e+04)))))

(event Game|Damage|EventAnyDamage
  (params (Damage :type Float%20%28single-precision%29) (DamageType :type Damage%20Type%20Object%20Reference) (InstigatedBy :type Controller%20Object%20Reference) (DamageCauser :type Actor%20Object%20Reference))
  (Variables|Default|SetCurrentHealth (Math|Float|Clamp(Float) (- (Variables|Default|GetCurrentHealth) Damage) 0.0 (Variables|Default|GetMaxHealth))))

(event Input|ActionEvents|InputActionEnablecameraroation
  (params (Key :type Key%20Structure))
  (:Pressed
    (Variables|Default|SetRMB true))
  (:Released
    (Variables|Default|SetRMB false)))

(event Input|AxisEvents|InputAxisLookupanddown
  (params (AxisValue :type Float%20%28single-precision%29))
  (if (Variables|Default|GetRMB)
    (Transformation|AddRelativeRotation (Variables|Default|GetCamera) (Math|Rotator|MakeRotator 0.0 AxisValue 0.0) false false)))

(event Input|AxisEvents|InputAxisLookleftandright
  (params (AxisValue :type Float%20%28single-precision%29))
  (if (Variables|Default|GetRMB)
    (Transformation|AddRelativeRotation (Variables|Default|GetCamera) (Math|Rotator|MakeRotator 0.0 0.0 AxisValue) false false)))

(event Custom|SetClimbing
  (params (Climbing :type Boolean) (ClimbingSpeed :type Float%20%28single-precision%29) (InterpSpeed :type Float%20%28single-precision%29) (SoundChange :type Boolean))
  ;[1 1 1] SetClimbing
  (Utilities|FlowControl|Sequence
    (:then_0
      (Variables|Default|SetBrake 0.0)
      (Variables|Default|SetAddingVelocityDuration 0.0))
    (:then_1
      (Variables|Default|SetClimbingSpeed (Math|Float|SelectFloat (Variables|Default|GetClimbingSpeed) ClimbingSpeed (== ClimbingSpeed -1.0)))
      (Variables|Default|SetClimbingInterpSpeed (Math|Float|SelectFloat 5e+01 InterpSpeed (== InterpSpeed -1.0)))
      (bind _output_get (Variables|Default|SetClimbing Climbing))
      (if _output_get ; Make sure to set only when 'Start'.\nOtherwise, it causes inconsistency
        (Variables|Default|SetClimbingUseSound SoundChange))
      (if (Variables|Default|GetClimbingUseSound)
        (if (Variables|Default|GetClimbing)
          (CallFunction|FadetoTracktoClimb 1.0)
          (else
            (CallFunction|FadetoClimbtoTrack 1.0)))))
    (:then_2
      (Variables|Default|SettxtMinSpeed (select (Variables|Default|GetClimbing) "Climbing" (Utilities|Text|ToText(Float) (Variables|Default|GetMinSpeed) "HalfToEven" false true 1 324 0 1))))))

(event Custom|SetBrake
  (params (Brake :type Float%20%28single-precision%29) (MinSpeed%20%28-1%20to%20keep%20current%29 :type Float%20%28single-precision%29))
  ;[1 1 1] SetBrake
  (Utilities|FlowControl|Sequence
    (:then_0
      (Variables|Default|SetAddingVelocityDuration 0.0)
      (if (Variables|Default|GetClimbing)
        (Variables|Default|SetClimbing false)
        (if (Variables|Default|GetClimbingUseSound)
          (CallFunction|FadetoClimbtoTrack 1.0))))
    (:then_1
      (Variables|Default|SetBrake Brake)
      (if (>= MinSpeed%20%28-1%20to%20keep%20current%29 0.0)
        (Variables|Default|SetMinSpeed MinSpeed%20%28-1%20to%20keep%20current%29)))))

(event Custom|FadeToClimbToTrack
  (params (FadeDuration :type Float%20%28single-precision%29))
  ;[1 1 1] Sound Fading
  (Audio|Components|Audio|FadeOut (Variables|Default|GetClimbingSound) FadeDuration 0.0 "Linear" :!class /Script/Engine.AudioComponent)
  (Audio|Components|Audio|FadeIn (Variables|Default|GetTrackSound) FadeDuration 1.0 0.0 "Linear" :!class /Script/Engine.AudioComponent))

(event Custom|FadeToTrackToClimb
  (params (FadeDuration :type Float%20%28single-precision%29))
  ;[1 1 1] Sound Fading
  (Audio|Components|Audio|FadeOut (Variables|Default|GetTrackSound) FadeDuration 0.0 "Linear" :!class /Script/Engine.AudioComponent)
  (Audio|Components|Audio|FadeIn (Variables|Default|GetClimbingSound) FadeDuration 1.0 0.0 "Linear" :!class /Script/Engine.AudioComponent))

(event Custom|AddVelocity
  (params (Velocity :type Float%20%28single-precision%29) (Duration%20%280%20to%20once%29 :type Float%20%28single-precision%29))
  ;[1 1 1] AddVelocity
  (Utilities|FlowControl|Sequence
    (:then_0
      (Variables|Default|SetBrake 0.0)
      (if (Variables|Default|GetClimbing)
        (Variables|Default|SetClimbing false)
        (if (Variables|Default|GetClimbingUseSound)
          (CallFunction|FadetoClimbtoTrack 1.0))))
    (:then_1
      (Variables|Default|SetAddingVelocity Velocity)
      (bind _output_get (Variables|Default|SetAddingVelocityDuration Duration%20%280%20to%20once%29))
      (Variables|Default|SetAddingVelocityPendingOnce (== _output_get 0.0)) ; This event was called at midst of Tick>Sequence.\nSo, AddingVelocity is overriden w/o adding at\nTick>Sequence1 if this bool is not used.
    )))

(event Custom|SetMinSpeed
  (params (MinSpeed :type Float%20%28single-precision%29))
  ;[1 1 1] MinSpeed
  (bind _output_get (Variables|Default|SetMinSpeed MinSpeed))
  (if (not (Variables|Default|GetClimbing))
    (Variables|Default|SettxtMinSpeed (Utilities|Text|ToText(Float) _output_get "HalfToEven" false true 1 324 0 1))))

(fn ConstructionScript
  (Variables|Default|SetMaxHealth (Variables|Default|GetMaxHealth)))

(fn GetPitch(1to1)
  (return (/ (- (Math|Float|Absolute(Float) (.pitch (Math|Rotator|Delta(Rotator) (Spline|GetRotationatDistanceAlongSpline (Variables|/Game/Assets/Rollercoaster/_Main/TrackSpline.TrackSpline_C|GetSpline (Variables|Default|GetSplineActor)) (Variables|Default|GetDistance) "World") "90.000000,0.000000, 0"))) 9e+01) 9e+01)))

(event EventTick
  (params (DeltaSeconds :type Float%20%28single-precision%29))
  (bind _tracksound (Variables|Default|GetTrackSound))
  (bind _minspeed (Variables|Default|GetMinSpeed))
  (Utilities|FlowControl|Sequence
    (:then_0
      ;[1 1 1] Calculate Speed and Distance
      (if (Variables|Default|GetClimbing)
        _
        (else
          (bind _output_get (Variables|Default|SetCurrentSpeed (+ (Variables|Default|GetCurrentSpeed) (|Gravity_2))))
          (Variables|Default|SetCurrentSpeed (+ _output_get (|AddVelocity__2) (|Brake__2)))
          (Variables|Default|SetAddingVelocityPendingOnce false)))
      (Variables|Default|SetDistance (|CalcDistance_2))
      (|SetActorLocation&Rotation_2))
    (:then_1
      (Utilities|FlowControl|Sequence
        (:then_0
          (if (> (Variables|Default|GetAddingVelocityDuration) 0.0)
            (Variables|Default|SetAddingVelocityDuration (- (Variables|Default|GetAddingVelocityDuration) (Utilities|Time|GetWorldDeltaSeconds)))
            (elif (not (Variables|Default|GetAddingVelocityPendingOnce))
              (Variables|Default|SetAddingVelocity 0.0)
              (Variables|Default|SetAddingVelocityDuration 0.0))))
        (:then_1
          ;[1 1 1] Brake
          (if (and (<= (Variables|Default|GetCurrentSpeed) (Variables|Default|GetMinSpeed)) (> (Variables|Default|GetBrake) 0.0))
            (Variables|Default|SetBrake 0.0)))
        (:then_2
          ;[1 1 1] Climbing
          (if (Variables|Default|GetClimbing)
            (if (!= (Variables|Default|GetCurrentSpeed) (Variables|Default|GetClimbingSpeed))
              (Variables|Default|SetCurrentSpeed (Math|Interpolation|FInterptoConstant (Variables|Default|GetCurrentSpeed) (Variables|Default|GetClimbingSpeed) (Utilities|Time|GetWorldDeltaSeconds) (Variables|Default|GetClimbingInterpSpeed))) ; Make close to Climbing speed
            )
            (else
              ;[1 1 1] CurrentSpeed < MinSpeed (while not climbing)
              (if (< (Variables|Default|GetCurrentSpeed) _minspeed)
                (Variables|Default|SetCurrentSpeed _minspeed)))))))
    (:then_2
      ;[1 1 1] Widget
      (Variables|Default|SettxtSpeed (Utilities|Text|ToText(Float) (Variables|Default|GetCurrentSpeed) "HalfToEven" false true 1 324 0 1))
      ;[1 1 1] Sound
      (Audio|Parameter|SetFloatParameter _tracksound "Speed" (Math|Float|Clamp(Float) (/ (Variables|Default|GetCurrentSpeed) 1e+02)) :!class /Script/Engine.AudioComponent)
      (Audio|Parameter|SetFloatParameter _tracksound "TrackLowVolume" (Math|Curves|GetFloatValue (Variables|Default|GetTrackLowVolume) (Math|Float|Clamp(Float) (/ (Variables|Default|GetCurrentSpeed) 1e+02))) :!class /Script/Engine.AudioComponent))))